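; Player sword actor that also runs the match's enemy waves and timed win condition.
; Tick snaps it beside the player pawn, choosing the side from mouse X against a fixed screen threshold.
; A looping Atkspeed timer spawns BP_Slash on that same side.
; Other BeginPlay timers repeatedly spawn Wave1Enemy batches at random edges of a box around the player, and after two minutes show BP_Win and pause the game.
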(event `self.ReceiveTick`
  (params (DeltaSeconds :type "Float (single-precision)"))
  (bind (_returnvalue_x _returnvalue_y _returnvalue_z) (`KismetMathLibrary.BreakVector` (`SceneComponent.K2_GetComponentLocation` (`Actor.RootComponent` (`GameplayStatics.GetPlayerPawn` 0)))))
  ;[1 1 1] Sword stays with player/mouse
  (bind _returnvalue (`WidgetLayoutLibrary.GetMousePositionOnPlatform`))
  (if (> (`KismetMathLibrary.BreakVector2D` _returnvalue) 766.0)
    (`self.K2_SetActorLocation` (`KismetMathLibrary.MakeVector` (- _returnvalue_x 30.0) _returnvalue_y _returnvalue_z))
    (else
      (`self.K2_SetActorLocation` (`KismetMathLibrary.MakeVector` (+ _returnvalue_x 30.0) _returnvalue_y _returnvalue_z)))))

(event `WIN`
  (bind _returnvalue (`|CreateWidget` "/Game/UI/BP_Win.BP_Win_C"))
  (`UserWidget.AddToViewport` _returnvalue 0)
  (`WidgetBlueprintLibrary.SetInputMode_UIOnlyEx` (`GameplayStatics.GetPlayerController` 0) null)
  (`GameplayStatics.SetGamePaused` true))

(event `self.ReceiveBeginPlay`
  ;[1 1 1] Basic Enemy Waves
  (`KismetSystemLibrary.K2_SetTimerDelegate` (delegate `WIN`) 120.0)
  (`KismetSystemLibrary.K2_SetTimerDelegate` (delegate `Spawn Basic Enemies`) 10.0 true)
  ;[1 1 1] Sword Basic Attack
  (`KismetSystemLibrary.K2_SetTimerDelegate` (delegate `Attack`) (`self.atkspeed`) true))

(event `Spawn Basic Enemies`
  (bind _returnvalue (`KismetMathLibrary.RandomBool`))
  (bind (_returnvalue_x _returnvalue_y _returnvalue_z) (`KismetMathLibrary.BreakVector` (`SceneComponent.K2_GetComponentLocation` (`Actor.RootComponent` (`GameplayStatics.GetPlayerPawn` 0)))))
  (bind (_returnvalue_x_2 _returnvalue_y_2 _returnvalue_z_2) (`KismetMathLibrary.BreakVector` (`SceneComponent.K2_GetComponentLocation` (`Actor.RootComponent` (`GameplayStatics.GetPlayerPawn` 0)))))
  ;[1 1 1] Basic Enemy Waves
  (for _ (range 4)
    (if (`KismetMathLibrary.RandomBool`)
      (if _returnvalue
        (`|SpawnActorFromClass` "/Game/Enemies/Wave1Enemy.Wave1Enemy_C" (`KismetMathLibrary.MakeTransform` (`KismetMathLibrary.MakeVector` (+ _returnvalue_x_2 (`KismetMathLibrary.RandomFloatInRange` -1000.0 1000.0)) (+ _returnvalue_y_2 750.0) _returnvalue_z_2)) "Undefined" "MultiplyWithRoot" null null)
        (else
          (`|SpawnActorFromClass` "/Game/Enemies/Wave1Enemy.Wave1Enemy_C" (`KismetMathLibrary.MakeTransform` (`KismetMathLibrary.MakeVector` (+ _returnvalue_x_2 (`KismetMathLibrary.RandomFloatInRange` -1000.0 1000.0)) (+ _returnvalue_y_2 -750.0) _returnvalue_z_2)) "Undefined" "MultiplyWithRoot" null null)))
      (elif _returnvalue
        (`|SpawnActorFromClass` "/Game/Enemies/Wave1Enemy.Wave1Enemy_C" (`KismetMathLibrary.MakeTransform` (`KismetMathLibrary.MakeVector` (+ _returnvalue_x -1000.0) (+ _returnvalue_y (`KismetMathLibrary.RandomFloatInRange` -750.0 750.0)) _returnvalue_z)) "Undefined" "MultiplyWithRoot" null null)
        (else
          (`|SpawnActorFromClass` "/Game/Enemies/Wave1Enemy.Wave1Enemy_C" (`KismetMathLibrary.MakeTransform` (`KismetMathLibrary.MakeVector` (+ _returnvalue_x 1000.0) (+ _returnvalue_y (`KismetMathLibrary.RandomFloatInRange` -750.0 750.0)) _returnvalue_z)) "Undefined" "MultiplyWithRoot" null null))))))

(event `Attack`
  (bind (_returnvalue_x _returnvalue_y _returnvalue_z) (`KismetMathLibrary.BreakVector` (`SceneComponent.K2_GetComponentLocation` (`Actor.RootComponent` (`GameplayStatics.GetPlayerPawn` 0)))))
  ;[1 1 1] Sword Basic Attack
  (bind _returnvalue (`WidgetLayoutLibrary.GetMousePositionOnPlatform`))
  (if (> (`KismetMathLibrary.BreakVector2D` _returnvalue) 766.0)
    (`|SpawnActorFromClass` "/Game/Weapons/BP_Slash.BP_Slash_C" (`KismetMathLibrary.MakeTransform` (`KismetMathLibrary.MakeVector` (- _returnvalue_x 100.0) _returnvalue_y _returnvalue_z) (struct :`Yaw` 180.0)) "Undefined" "MultiplyWithRoot" null null)
    (else
      (`|SpawnActorFromClass` "/Game/Weapons/BP_Slash.BP_Slash_C" (`KismetMathLibrary.MakeTransform` (`KismetMathLibrary.MakeVector` (+ _returnvalue_x 100.0) _returnvalue_y _returnvalue_z)) "Undefined" "MultiplyWithRoot" null null))))

(fn `UserConstructionScript`)