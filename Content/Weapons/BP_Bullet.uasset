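; BP_Bullet is a Character-based sprite projectile that damages overlapped actors tagged "enemy".
; On spawn it takes a direction from the cursor's offset to screen centre, then sustains movement by feeding velocity back as movement input.
; It reads speed, pierce, damage, crit and explosion settings from BP_Blaster.
; Crits randomly double damage with a sound; exhausted pierce destroys it, optionally spawning BP_Explosion, and a timer limits its lifetime.
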(event `self.ReceiveBeginPlay`
  (bind (_returnvalue_x _returnvalue_y) (`KismetMathLibrary.BreakVector2D` (`WidgetLayoutLibrary.GetViewportSize`)))
  (bind (_locationx _locationy) (`PlayerController.GetMousePosition` (`GameplayStatics.GetPlayerController` 0)))
  (bind _output_get (set `self.unitvector` (`KismetMathLibrary.MakeVector` (- (/ _returnvalue_x 2.0) _locationx) (- (/ _returnvalue_y 2.0) _locationy))))
  (`self.AddMovementInput` _output_get)
  (bind _returnvalue (`GameplayStatics.GetActorOfClass` "/Game/Weapons/BP_Blaster.BP_Blaster_C"))
  (bind _output_get_2 (set `self.bpblaster` _returnvalue))
  (`KismetSystemLibrary.K2_SetTimerDelegate` (delegate `BYE`) 5.0)
  (set `self.pierced` (`/Game/Weapons/BP_Blaster.pierce` _output_get_2))
  (set `CharacterMovementComponent.MaxWalkSpeed` (`/Game/Weapons/BP_Blaster.speed` _output_get_2) (`self.CharacterMovement`)))

(event `self.ReceiveTick`
  (params (DeltaSeconds :type "Float (single-precision)"))
  (`self.AddMovementInput` (`self.GetVelocity`)))

(event `BYE`
  (`self.K2_DestroyActor`))

(event `self.bullet-01_Sprite.OnComponentBeginOverlap`
  (params (OverlappedComponent :type "PrimitiveComponent Object Reference") (OtherActor :type "Actor Object Reference") (OtherComp :type "PrimitiveComponent Object Reference") (OtherBodyIndex :type Integer) (bFromSweep :type Boolean) (SweepResult :type "HitResult Structure (by ref)"))
  (bind _returnvalue (`self.K2_GetActorLocation`))
  (bind _bpblaster (`self.bpblaster`))
  (bind _returnvalue_2 (- (`self.pierced`) 1.0))
  (bind _damage (`/Game/Weapons/BP_Blaster.damage` _bpblaster))
  (if (`self.ActorHasTag` OtherActor "enemy")
    (if (`/Game/Weapons/BP_Blaster.crits` _bpblaster)
      (if (>= (`KismetMathLibrary.RandomFloatInRange` 0.0 100.0) 20.0)
        (`GameplayStatics.ApplyDamage` OtherActor _damage :!label _label)
        (else
          (`GameplayStatics.ApplyDamage` OtherActor (* _damage 2.0))
          (`GameplayStatics.PlaySoundAtLocation` "/Game/Weapons/valorant-headshot-101soundboards.valorant-headshot-101soundboards" _returnvalue (struct) 5.0 1.0 0.0 null null null null)))
      (else
        (goto _label)))
    (if (<= _returnvalue_2 0.0)
      (if (`/Game/Weapons/BP_Blaster.explosions` _bpblaster)
        (`|SpawnActorFromClass` "/Game/Weapons/BP_Explosion.BP_Explosion_C" (`KismetMathLibrary.MakeTransform` _returnvalue) "Undefined" "MultiplyWithRoot" null null))
      (`self.K2_DestroyActor`)
      (else
        (set `self.pierced` _returnvalue_2)))))

(fn `UserConstructionScript`)