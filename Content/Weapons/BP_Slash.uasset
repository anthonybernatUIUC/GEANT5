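; BP_Slash is a short-lived sword slash hitbox that damages overlapped actors tagged "enemy" and destroys itself on a timer a fraction of a second after spawning.
; It finds BP_Sword on BeginPlay, reading its damage and critical flag on hit and scaling the slash sprite by its Aoe value every Tick.
; When the sword's Critical flag is set, a random roll can double the damage and play a critical-hit sound.
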(event `self.ReceiveBeginPlay`
  (bind _returnvalue (`GameplayStatics.GetActorOfClass` "/Game/Weapons/BP_Sword.BP_Sword_C"))
  (set `self.bpsword` _returnvalue)
  (`KismetSystemLibrary.K2_SetTimerDelegate` (delegate `Bye`) 0.125))

(event `Bye`
  (`self.K2_DestroyActor`))

(event `self.ReceiveTick`
  (params (DeltaSeconds :type "Float (single-precision)"))
  (bind _aoe (`/Game/Weapons/BP_Sword.aoe` (`self.bpsword`)))
  (`SceneComponent.SetWorldScale3D` (`self.slash-01_Sprite`) (`KismetMathLibrary.MakeVector` _aoe _aoe _aoe)))

(event `self.slash-01_Sprite.OnComponentBeginOverlap`
  (params (OverlappedComponent :type "PrimitiveComponent Object Reference") (OtherActor :type "Actor Object Reference") (OtherComp :type "PrimitiveComponent Object Reference") (OtherBodyIndex :type Integer) (bFromSweep :type Boolean) (SweepResult :type "HitResult Structure (by ref)"))
  (bind _bpsword (`self.bpsword`))
  (bind _damage (`/Game/Weapons/BP_Sword.damage` _bpsword))
  (if (`self.ActorHasTag` OtherActor "enemy")
    (if (`/Game/Weapons/BP_Sword.critical` _bpsword)
      (if (>= (`KismetMathLibrary.RandomFloatInRange` 0.0 100.0) 20.0)
        (`GameplayStatics.ApplyDamage` OtherActor _damage :!label _label)
        (else
          (`GameplayStatics.ApplyDamage` OtherActor (* _damage 2.0))
          (`GameplayStatics.PlaySoundAtLocation` "/Game/Weapons/brave-criticalhit-c03-101soundboards.brave-criticalhit-c03-101soundboards" (`self.K2_GetActorLocation`) (struct) 1.0 1.0 0.0 null null null null)))
      (else
        (goto _label)))))

(fn `UserConstructionScript`)