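; BP_Blaster is an auto-firing weapon actor that follows the player pawn.
; Each Tick it sits at a fixed X offset from the pawn, switching sides according to which half of the viewport the mouse is in.
; A looping timer set by Atkspeed spawns BP_Bullet at the pawn's location, not the blaster's, and plays a sound.
; Multishot spawns two bullets at that same point instead of one.
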(event `self.ReceiveTick`
  (params (DeltaSeconds :type "Float (single-precision)"))
  (bind _returnvalue_x (`KismetMathLibrary.BreakVector2D` (`WidgetLayoutLibrary.GetViewportSize`)))
  (bind (_returnvalue_x_2 _returnvalue_y _returnvalue_z) (`KismetMathLibrary.BreakVector` (`SceneComponent.K2_GetComponentLocation` (`Actor.RootComponent` (`GameplayStatics.GetPlayerPawn` 0)))))
  (if (> (`PlayerController.GetMousePosition` (`GameplayStatics.GetPlayerController` 0)) (* _returnvalue_x 0.5))
    (`self.K2_SetActorLocation` (`KismetMathLibrary.MakeVector` (- _returnvalue_x_2 30.0) _returnvalue_y _returnvalue_z))
    (else
      (`self.K2_SetActorLocation` (`KismetMathLibrary.MakeVector` (+ _returnvalue_x_2 30.0) _returnvalue_y _returnvalue_z)))))

(event `self.ReceiveBeginPlay`
  (`KismetSystemLibrary.K2_SetTimerDelegate` (delegate `Attack`) (`self.atkspeed`) true))

(event `Attack`
  (bind _returnvalue (`SceneComponent.K2_GetComponentLocation` (`Actor.RootComponent` (`GameplayStatics.GetPlayerPawn` 0))))
  (if (`self.multishot`)
    (`|SpawnActorFromClass` "/Game/Weapons/BP_Bullet.BP_Bullet_C" (`KismetMathLibrary.MakeTransform` _returnvalue) "AlwaysSpawn" "MultiplyWithRoot" null null)
    (`|SpawnActorFromClass` "/Game/Weapons/BP_Bullet.BP_Bullet_C" (`KismetMathLibrary.MakeTransform` _returnvalue) "AlwaysSpawn" "MultiplyWithRoot" null null)
    (else
      (`|SpawnActorFromClass` "/Game/Weapons/BP_Bullet.BP_Bullet_C" (`KismetMathLibrary.MakeTransform` _returnvalue) "AlwaysSpawn" "MultiplyWithRoot" null null)))
  (`GameplayStatics.PlaySoundAtLocation` "/Game/Weapons/Item_41.Item_41" (`self.K2_GetActorLocation`) (struct) 1.0 1.0 0.0 null null null null))

(fn `UserConstructionScript`)